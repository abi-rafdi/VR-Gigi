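; Resonant button Blueprint that sinks when a VR pawn overlaps it and rises back when the overlap ends.
; BeginPlay caches the start position; the Box's begin overlap and the Button's own end overlap drive MoveComponentTo on the Button.
; Tick uses height thresholds to fire and reset a DoOnce, which triggers nothing.
; The percussion abdomen sequence and resonant sound logic are disconnected and never run.
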(event OnComponentBeginOverlap(Box)
  (params (OverlappedComponent :type Primitive%20Component%20Object%20Reference) (OtherActor :type Actor%20Object%20Reference) (OtherComp :type Primitive%20Component%20Object%20Reference) (OtherBodyIndex :type Integer) (bFromSweep :type Boolean) (SweepResult :type Hit%20Result%20Structure%20%28by%20ref%29))
  ;[1 1 1] On Player Overlap, Push Button Down
  (Utilities|Casting|CastToVRPawn OtherActor)
  (Components|MoveComponentTo (Variables|Default|GetButton) (Math|Vector|MakeVector 0.0 0.0 (- (.z (Variables|Default|GetButtonStartPosition)) 1e+01)) "0, 0, 0" false false 0.2 false))

(event OnComponentEndOverlap(Button)
  (params (OverlappedComponent :type Primitive%20Component%20Object%20Reference) (OtherActor :type Actor%20Object%20Reference) (OtherComp :type Primitive%20Component%20Object%20Reference) (OtherBodyIndex :type Integer))
  ;[1 1 1] On Player End Overlap, Push Return to Start Position
  (Utilities|Casting|CastToVRPawn OtherActor)
  (Components|MoveComponentTo (Variables|Default|GetButton) (Math|Vector|MakeVector 0.0 0.0 (.z (Variables|Default|GetButtonStartPosition))) "0, 0, 0" false false 0.2 false))

(event EventBeginPlay
  ;[1 1 1] Set Button Start Location
  (Variables|Default|SetButtonStartPosition (Variables|/Script/Engine.SceneComponent|GetRelativeLocation (Variables|Default|GetButton))))

(event EventTick
  (params (DeltaSeconds :type Float%20%28single-precision%29))
  (bind _button (Variables|Default|GetButton))
  (bind _relativelocation (Variables|/Script/Engine.SceneComponent|GetRelativeLocation _button))
  ;[1 1 1] Play Sound when the button pressed, reset sound when the button returns to start position.
  (if (<= (.z _relativelocation) 6.0)
    (Utilities|FlowControl|DoOnce false :!label _label)
    (elif (>= (.z _relativelocation) 14.0)
      (goto _label Reset))))

(fn ConstructionScript)