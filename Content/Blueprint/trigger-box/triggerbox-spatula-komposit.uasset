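; Trigger box for the composite spatula step, which advances the game to the 11-CuringLight level.
; Its Gunting and TextRender components start hidden, show when a bp-spatula-komposit actor overlaps the box, and hide when that overlap ends.
; The overlap also starts parallel delays that destroy the spatula, play Spatulakomposit10 on the found LevelSequenceActor, then open the next level.
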(event OnComponentBeginOverlap(Box)
  (params (OverlappedComponent :type Primitive%20Component%20Object%20Reference) (OtherActor :type Actor%20Object%20Reference) (OtherComp :type Primitive%20Component%20Object%20Reference) (OtherBodyIndex :type Integer) (bFromSweep :type Boolean) (SweepResult :type Hit%20Result%20Structure%20%28by%20ref%29))
  (bind _asbp_spatula_komposit (Utilities|Casting|CastTobp-spatula-komposit OtherActor))
  (Utilities|FlowControl|Sequence
    (:then_0
      (CallFunction|ChangeComponentVisibility true))
    (:then_1
      (Utilities|FlowControl|Delay 1.0)
      (Actor|DestroyActor _asbp_spatula_komposit))
    (:then_2
      (Utilities|FlowControl|Delay 2.0)
      ;[1 1 1] Play AntisepticAnimation
      (bind _returnvalue (Actor|GetActorOfClass "/Script/LevelSequence.LevelSequenceActor"))
      (Class|LevelSequenceActor|SetSequence _returnvalue "/Game/Assets/Sequence/spatula-komposit10.spatula-komposit10")
      (Sequencer|Player|Play (Variables|/Script/LevelSequence.LevelSequenceActor|GetSequencePlayer _returnvalue) :!class /Script/MovieScene.MovieSceneSequencePlayer))
    (:then_3
      (Utilities|FlowControl|Delay 7.0)
      (Game|OpenLevel(byName) "11-CuringLight"))))

(event OnComponentEndOverlap(Box)
  (params (OverlappedComponent :type Primitive%20Component%20Object%20Reference) (OtherActor :type Actor%20Object%20Reference) (OtherComp :type Primitive%20Component%20Object%20Reference) (OtherBodyIndex :type Integer))
  (Utilities|Casting|CastTobp-spatula-komposit OtherActor)
  (CallFunction|ChangeComponentVisibility false))

(event Custom|ChangeComponentVisibility
  (params (Visible? :type Boolean))
  (Rendering|SetVisibility (Variables|Default|GetGunting) Visible? (Variables|Default|GetPropagate%20to%20Children)))

(event EventBeginPlay
  (CallFunction|ChangeComponentVisibility false))

(event Collision|EventActorBeginOverlap
  (params (OtherActor :type Actor%20Object%20Reference)))

(event EventTick
  (params (DeltaSeconds :type Float%20%28single-precision%29)))

(fn ConstructionScript)